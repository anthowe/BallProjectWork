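; TablePawn is a pawn that tilts its table mesh in response to player input.
; LookUp feeds controller pitch, while Turn feeds controller roll.
; Releasing Pitch sets the mesh's world rotation through PitchInput, which adds PitchValue to current pitch, zeroes roll and yaw, and ignores its UpOrDown argument.
; It also sets CanPress, which nothing here reads; an alternative additive-rotation chain is disconnected.
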(event EventBeginPlay)

(event Collision|EventActorBeginOverlap
  (params (OtherActor :type Actor%20Object%20Reference)))

(event EventTick
  (params (DeltaSeconds :type Float%20%28single-precision%29)))

(event Input|ActionEvents|InputActionPitch
  (params (Key :type Key%20Structure))
  (:Released
    (bind _returnvalue (CallFunction|PitchInput -1))
    (Transformation|SetWorldRotation (Variables|Default|GetTableMesh) _returnvalue false false)
    (Variables|Default|SetCanPress true)))

(event Input|AxisEvents|InputAxisLookUp
  (params (AxisValue :type Float%20%28single-precision%29))
  (Pawn|Input|AddControllerPitchInput AxisValue))

(event Input|AxisEvents|InputAxisTurn
  (params (AxisValue :type Float%20%28single-precision%29))
  (Pawn|Input|AddControllerRollInput AxisValue))

(fn ConstructionScript)

(fn PitchInput
  (params (Up%20Or%20Down :type Integer))
  (return (Math|Rotator|MakeRotator 0.0 (+ (Variables|Default|GetPitchValue) (.Pitch (Math|Rotator|BreakRotator (Transformation|GetWorldRotation (Variables|Default|GetTableMesh))))) 0.0)))
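; BallPawnBP is a physics-driven ball pawn that rolls and jumps.
; Movement axes apply torque to BallMesh, while jumping applies a vertical velocity-change impulse, locked until the next Hit event re-enables it.
; On actor overlap, it loops through CollisionSphere's overlapping actors, applying radial force to StaticMeshActors and a fixed-direction kick to the ball for each one.
; The loop body depends on a cast to StaticMeshActor.
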(event Collision|EventHit
  (params (MyComp :type Primitive%20Component%20Object%20Reference) (Other :type Actor%20Object%20Reference) (OtherComp :type Primitive%20Component%20Object%20Reference) (bSelfMoved :type Boolean) (HitLocation :type Vector :default "0, 0, 0") (HitNormal :type Vector :default "0, 0, 0") (NormalImpulse :type Vector :default "0, 0, 0") (Hit :type Hit%20Result%20Structure%20%28by%20ref%29))
  (Variables|Default|SetCanJump true))

(event Collision|EventActorBeginOverlap
  (params (OtherActor :type Actor%20Object%20Reference))
  (for _array_element (Collision|GetOverlappingActors (Variables|Default|GetCollisionSphere) 0 :!class /Script/Engine.PrimitiveComponent)
    (bind _asstatic_mesh_actor (Utilities|Casting|CastToStaticMeshActor _array_element))
    (Physics|AddRadialForce (Variables|/Script/Engine.StaticMeshActor|GetStaticMeshComponent _asstatic_mesh_actor) (Transformation|GetActorLocation) 2e+03 (Variables|Default|GetCollisionForce) "RIF_Constant" true)
    (Physics|AddForce (Variables|Default|GetBallMesh) (Math|Vector|MakeVector (* (Variables|Default|GetCollisionForce) -0.2) 6e+04 2.5e+03) "None" true)))

(event Input|ActionEvents|InputActionJump
  (params (Key :type Key%20Structure))
  (:Pressed
    (if (Variables|Default|GetCanJump)
      (Physics|AddImpulse (Variables|Default|GetBallMesh) (Math|Vector|MakeVector 0.0 0.0 (Variables|Default|GetJumpForce)) "None" true)
      (Variables|Default|SetCanJump false))))

(event Input|AxisEvents|InputAxisMoveForward
  (params (AxisValue :type Float%20%28single-precision%29))
  (Class|PrimitiveComponent|AddTorqueinDegrees (Variables|Default|GetBallMesh) (Math|Vector|MakeVector 0.0 (* AxisValue (Variables|Default|GetTorque)) 0.0) "None" true))

(event Input|AxisEvents|InputAxisMoveRight
  (params (AxisValue :type Float%20%28single-precision%29))
  (Class|PrimitiveComponent|AddTorqueinDegrees (Variables|Default|GetBallMesh) (Math|Vector|MakeVector (* AxisValue (Variables|Default|GetTorque) -1.0) 0.0 0.0) "None" true))

(fn ConstructionScript)